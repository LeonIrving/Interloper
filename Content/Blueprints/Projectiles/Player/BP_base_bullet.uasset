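; Base player projectile Blueprint that deals damage on hit and destroys itself after a set lifetime.
; An area-of-effect flag switches between single-target damage on the hit actor and radial damage with falloff around the impact.
; The area branch also spawns a scaled explosion emitter and plays an attenuated sound.
; Both hit branches and the lifetime timeout end in destroying the actor.
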(event EventBeginPlay
  (Utilities|FlowControl|Delay (Variables|Default|GetLifetime))
  (Actor|DestroyActor))

(event Collision|EventHit
  (params (MyComp :type Primitive%20Component%20Object%20Reference) (Other :type Actor%20Object%20Reference) (OtherComp :type Primitive%20Component%20Object%20Reference) (bSelfMoved :type Boolean) (HitLocation :type Vector :default "0, 0, 0") (HitNormal :type Vector :default "0, 0, 0") (NormalImpulse :type Vector :default "0, 0, 0") (Hit :type Hit%20Result%20Structure%20%28by%20ref%29))
  (bind _returnvalue (Transformation|GetActorLocation))
  (bind _self self)
  (bind _damage (Variables|Default|GetDamage))
  (if (Variables|Default|GetisAreaOfEffect)
    (Class|GameplayStatics|ApplyRadialDamagewithFalloff _damage 1.0 _returnvalue (Variables|Default|GetAOE%20InnerRadius) (Variables|Default|GetAOE%20OuterRadius) (Variables|Default|GetAOE%20DamageFalloff) 0 0 _self 0 "ECC_Visibility")
    (Effects|SpawnEmitteratLocation (Variables|Default|GetExplosion) _returnvalue "0, 0, 0" (Variables|Default|GetExplosionScale))
    (Audio|PlaySoundatLocation (Variables|Default|GetExplosionSound) _returnvalue "0, 0, 0" 1.0 1.0 0.0 "/Game/Audio/SA_explosion.SA_explosion" 0 0)
    (else
      (Game|Damage|ApplyDamage Other _damage 0 _self)))
  (Actor|DestroyActor))

(fn ConstructionScript)