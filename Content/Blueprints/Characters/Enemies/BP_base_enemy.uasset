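; Base enemy that detects the player by pawn sensing, then attacks with radial melee damage or spawned projectiles, as set by IsMelee.
; Melee and mobile ranged enemies move into AttackRange before attacking, while HoldsPosition ranged ones fire in place, with a delay gating each attack.
; Once the player is seen, Tick yaws the body and aims BulletSpawn at them.
; Damage updates a health bar widget, and lethal damage triggers an explosion and destroys the actor.
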(event OnSeePawn(PawnSensing)
  (params (Pawn :type Pawn%20Object%20Reference))
  (bind _returnvalue (Transformation|GetActorLocation))
  (bind _self self)
  (bind _bulletspawn (Variables|Default|GetBulletSpawn))
  (bind _target (Variables|Default|GetTarget))
  (bind _attackrange (Variables|Default|GetAttackRange))
  (bind _returnvalue_2 (Transformation|GetWorldTransform _bulletspawn))
  (bind _asfirst_person_character (Utilities|Casting|CastToFirstPersonCharacter Pawn))
  (Variables|Default|SetPlayer _asfirst_person_character)
  (Variables|Default|SetSeesPlayer true)
  (if (Variables|Default|GetisMelee)
    ;[0 0 0] Melee Attack
    (AI|AIMoveTo _self _target (Variables|Default|GetPlayer) _attackrange false
      (:OnSuccess
        (if (Variables|Default|GetCanAttack)
          (Game|Damage|ApplyRadialDamage (Variables|Default|GetDamage) _returnvalue 2e+02 0 0 _self 0 false "ECC_Visibility")
          (Audio|PlaySoundatLocation (Variables|Default|GetAttackSound) _returnvalue "0, 0, 0" 1.0 1.0 0.0 "/Game/Audio/SA_enemy.SA_enemy" 0 0)
          (Variables|Default|SetCanAttack false)
          (Utilities|FlowControl|Delay (Variables|Default|GetAttackDelay))
          (Variables|Default|SetCanAttack true))))
    (else
      ;[0 0 0] Ranged Attack
      (if (Variables|Default|GetHoldsPosition)
        _
        (else
          (AI|AIMoveTo _self _target (Variables|Default|GetPlayer) _attackrange false
            (:OnSuccess
              _))))
      (if (Variables|Default|GetCanAttack)
        (Game|SpawnActorfromClass (Variables|Default|GetProjectile) (Math|Transform|MakeTransform (.location _returnvalue_2) (.rotation _returnvalue_2) "1,1,1") "Undefined" 0 0)
        (Audio|PlaySoundatLocation (Variables|Default|GetAttackSound) (.location _returnvalue_2) "0, 0, 0" 1.0 1.0 0.0 "/Game/Audio/SA_enemy.SA_enemy" 0 0)
        (Variables|Default|SetCanAttack false)
        (Utilities|FlowControl|Delay (Variables|Default|GetAttackDelay))
        (Variables|Default|SetCanAttack true)))))

(event EventTick
  (params (DeltaSeconds :type Float%20%28single-precision%29))
  (Variables|Default|SetDeltaSeconds DeltaSeconds)
  (bind _asfirst_person_character (Utilities|Casting|CastToFirstPersonCharacter (Game|GetPlayerCharacter 0)))
  (Variables|Default|SetTarget (Variables|/Game/Blueprints/Characters/FirstPersonCharacter.FirstPersonCharacter_C|GetPlayerTarget _asfirst_person_character))
  (if (Variables|Default|GetSeesPlayer)
    (CallFunction|LookatTarget)))

(event EventBeginPlay
  (Variables|Default|SetHealth (Variables|Default|GetMaxHealth))
  (bind _asui_enemy_health (Utilities|Casting|CastToUI_enemy_health (UserInterface|GetUserWidgetObject (Variables|Default|GetHealthbar))))
  (bind _output_get (Variables|Default|SetHealthbarWidget _asui_enemy_health))
  (Variables|/Game/Blueprints/Characters/Enemies/UI_enemy_health.UI_enemy_health_C|SetMaxValue _output_get (Variables|Default|GetMaxHealth))
  (Variables|/Game/Blueprints/Characters/Enemies/UI_enemy_health.UI_enemy_health_C|SetValue _output_get (Variables|Default|GetHealth)))

(event Game|Damage|EventAnyDamage
  (params (Damage :type Float%20%28single-precision%29) (DamageType :type Damage%20Type%20Object%20Reference) (InstigatedBy :type Controller%20Object%20Reference) (DamageCauser :type Actor%20Object%20Reference))
  ;[0 0 0] Take Damage
  (if (>= Damage (Variables|Default|GetHealth))
    (CallFunction|Death)
    (else
      (bind _output_get (Variables|Default|SetHealth (- (Variables|Default|GetHealth) Damage)))
      (Variables|/Game/Blueprints/Characters/Enemies/UI_enemy_health.UI_enemy_health_C|SetValue (Variables|Default|GetHealthbarWidget) _output_get))))

(fn ConstructionScript)

(fn Death
  (bind _returnvalue (Transformation|GetActorTransform))
  (Effects|SpawnEmitteratLocation "/Game/Particles/P_Explosion2.P_Explosion2" (.location _returnvalue) (.rotation _returnvalue))
  (Audio|PlaySoundatLocation "/Game/Audio/Effects/C_Small_Explosion.C_Small_Explosion" (.location _returnvalue) "0, 0, 0" 1.0 1.0 0.0 "/Game/Audio/SA_enemy.SA_enemy" 0 0)
  (Actor|DestroyActor))

(fn LookatTarget
  (bind _bulletspawn (Variables|Default|GetBulletSpawn))
  (bind _returnvalue (Transformation|GetWorldTransform _bulletspawn))
  (Transformation|SetActorRotation (Math|Interpolation|RInterpTo (Transformation|GetActorRotation) (Math|Rotator|MakeRotator 0.0 0.0 (.yaw (Math|Rotator|FindLookatRotation (Transformation|GetActorLocation) (Transformation|GetActorLocation (Variables|Default|GetPlayer))))) (Variables|Default|GetDeltaSeconds) 1e+02))
  (Transformation|SetWorldRotation _bulletspawn (Math|Interpolation|RInterpTo (.rotation _returnvalue) (Math|Rotator|FindLookatRotation (.location _returnvalue) (Transformation|GetActorLocation (Variables|Default|GetPlayer))) (Variables|Default|GetDeltaSeconds) 1e+02) false false))