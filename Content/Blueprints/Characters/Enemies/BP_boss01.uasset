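; Boss enemy that chases the player on sight and fires at them with two guns.
; Pawn sensing starts an AI move toward the player, aims both guns and triggers two delayed Attack volleys, each spawning bullets with sound.
; Damage lowers Health, but the death sequence (hide, explode, destroy) is not connected to any event, and Tick only casts the player character.
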(event OnSeePawn(PawnSensing)
  (params (Pawn :type Pawn%20Object%20Reference))
  (bind _gun2 (Variables|Default|Getgun2))
  (bind _gun1 (Variables|Default|Getgun1))
  ;[1 1 1] AI
  (if (not (Variables|Default|GetisDead))
    (bind _asfirst_person_character (Utilities|Casting|CastToFirstPersonCharacter Pawn))
    (bind _output_get (Variables|Default|SetPlayerCharacterReference _asfirst_person_character))
    (AI|AIMoveTo self "0, 0, 0" _output_get 2e+03 false
      (:then
        ;[1 1 1] Attacking
        (Transformation|SetWorldRotation _gun1 (Math|Rotator|FindLookatRotation (Transformation|GetWorldLocation _gun1) (Transformation|GetWorldLocation (Variables|/Script/Engine.Actor|GetRootComponent (Variables|Default|GetPlayerCharacterReference)))) false false)
        (Transformation|SetWorldRotation _gun2 (Math|Rotator|FindLookatRotation (Transformation|GetWorldLocation _gun2) (Transformation|GetWorldLocation (Variables|/Script/Engine.Actor|GetRootComponent (Variables|Default|GetPlayerCharacterReference)))) false false)
        (Utilities|FlowControl|Delay 1.0)
        (CallFunction|Attack)
        (Utilities|FlowControl|Delay 1.0)
        (CallFunction|Attack)))))

(event EventTick
  (params (DeltaSeconds :type Float%20%28single-precision%29))
  ;[1 1 1] Taking Damage
  (bind _asfirst_person_character (Utilities|Casting|CastToFirstPersonCharacter (Game|GetPlayerCharacter 0))))

(event Game|Damage|EventAnyDamage
  (params (Damage :type Float%20%28single-precision%29) (DamageType :type Damage%20Type%20Object%20Reference) (InstigatedBy :type Controller%20Object%20Reference) (DamageCauser :type Actor%20Object%20Reference))
  ;[1 1 1] Taking Damage
  (Variables|Default|SetHealth (- (Variables|Default|GetHealth) Damage)))

(fn ConstructionScript)

(fn Attack
  (bind _gun1 (Variables|Default|Getgun1))
  (bind _gun2 (Variables|Default|Getgun2))
  (bind _returnvalue (Transformation|GetWorldTransform _gun2))
  (bind _returnvalue_2 (Transformation|GetWorldTransform _gun1))
  (if (not (Variables|Default|GetisDead))
    (Game|SpawnActorfromClass "/Game/Blueprints/Projectiles/BP_enemyBullet01.BP_enemyBullet01_C" (Math|Transform|MakeTransform (.location _returnvalue_2) (.rotation _returnvalue_2) (Variables|Default|GetBulletSpawnScale)) "Undefined" 0 0)
    (Audio|PlaySoundatLocation "/Game/Audio/Effects/C_shoot01.C_shoot01" (Transformation|GetWorldLocation _gun1) "0, 0, 0" 0.5 0.7 0.0 0 0 0)
    (Game|SpawnActorfromClass "/Game/Blueprints/Projectiles/BP_enemyBullet01.BP_enemyBullet01_C" (Math|Transform|MakeTransform (.location _returnvalue) (.rotation _returnvalue) (Variables|Default|GetBulletSpawnScale)) "Undefined" 0 0)
    (Audio|PlaySoundatLocation "/Game/Audio/Effects/C_shoot01.C_shoot01" (Transformation|GetWorldLocation _gun2) "0, 0, 0" 0.5 0.7 0.0 0 0 0)))