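; Mech boss enemy that ends level 3 when destroyed.
; On seeing the player, it interpolates turret yaw and gun pitch toward them, fires delayed projectiles from two barrels and creates a boss health bar.
; Damage updates the bar and plays a throttled hitmarker, while player death resets boss health.
; Death spawns a hub portal and waypoint, marks Level3Complete on the game instance, then explodes and destroys the actor.
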(event OnSeePawn(PawnSensing)
  (params (Pawn :type Pawn%20Object%20Reference))
  (Utilities|Casting|CastToFirstPersonCharacter Pawn)
  (if (not (Variables|Default|GetIsDead))
    (CallFunction|RotateTurret)
    (CallFunction|TurretAttack)
    (CallFunction|ShowHealthBar)))

(event Custom|Hit%20Sound
  (Utilities|FlowControl|DoOnce false :!label _label
    (:Completed
      (Audio|PlaySound2D "/Game/Audio/Effects/Guns/A_Hitmarker.A_Hitmarker" 1.0 1.0 0.0 0 0)
      (Utilities|FlowControl|Delay 0.1)
      (goto _label Reset))))

(event Custom|Rotate%20Turret
  (bind _deltaseconds (Variables|Default|GetDeltaSeconds))
  (bind _guns (Variables|Default|GetGuns))
  (bind _turret (Variables|Default|GetTurret))
  (bind _asfirst_person_character (Utilities|Casting|CastToFirstPersonCharacter (Game|GetPlayerCharacter 0)))
  (Transformation|SetWorldRotation _turret (Math|Rotator|MakeRotator 0.0 0.0 (.yaw (Math|Interpolation|RInterpTo (Transformation|GetWorldRotation _turret) (Math|Rotator|FindLookatRotation (Transformation|GetWorldLocation _turret) (Transformation|GetActorLocation _asfirst_person_character)) _deltaseconds 2.0))) false false)
  (Transformation|SetRelativeRotation _guns (Math|Rotator|MakeRotator 0.0 (.pitch (Math|Interpolation|RInterpTo (Transformation|GetWorldRotation _guns) (Math|Rotator|FindLookatRotation (Transformation|GetWorldLocation _guns) (Transformation|GetActorLocation _asfirst_person_character)) _deltaseconds 25.0)) 0.0) false false))

(event Custom|Death
  (bind _returnvalue (Transformation|GetActorTransform))
  (bind _returnvalue_2 (+ (.z (.location _returnvalue)) -1e+03))
  (Utilities|FlowControl|DoOnce false
    (:Completed
      (bind _returnvalue_3 (Game|SpawnActorfromClass "/Game/Blueprints/Environment/Doors/BP_level_portal_sphere.BP_level_portal_sphere_C" (Math|Transform|MakeTransform (Math|Vector|MakeVector (.x (.location _returnvalue)) (.y (.location _returnvalue)) _returnvalue_2) (.rotation _returnvalue) "10.000000,10.000000,10.000000") "Undefined" 0 0))
      (bind _output_get (Variables|Default|SetDeath%20Portal _returnvalue_3))
      (Variables|/Game/Blueprints/Environment/Doors/BP_level_portal_sphere.BP_level_portal_sphere_C|SetLevelToLoad _output_get "Hub")
      (Variables|/Game/Blueprints/Environment/Doors/BP_level_portal_sphere.BP_level_portal_sphere_C|SetLevel%20Name _output_get "The Terminus")
      (Variables|/Game/Blueprints/Environment/Doors/BP_level_portal_sphere.BP_level_portal_sphere_C|SetLevel%20Image _output_get "/Game/Textures/T_Hub_Image.T_Hub_Image")
      (Game|SpawnActorfromClass "/Game/Blueprints/Objectives/BP_single_waypoint.BP_single_waypoint_C" (Math|Transform|MakeTransform (Math|Vector|MakeVector (.x (.location _returnvalue)) (.y (.location _returnvalue)) _returnvalue_2) (.rotation _returnvalue) "1,1,1") "Undefined" 0 0)
      (bind _asinterloper_game_instance (Utilities|Casting|CastToInterloperGameInstance (Game|GetGameInstance)))
      (Variables|/Game/Blueprints/InterloperGameInstance.InterloperGameInstance_C|SetLevel3Complete _asinterloper_game_instance true)
      (Effects|SpawnEmitteratLocation "/Game/Particles/P_Explosion2.P_Explosion2" (Transformation|GetActorLocation) "0, 0, 0" "10.000000,10.000000,10.000000")
      (Actor|DestroyActor))))

(event Custom|Reset
  (bind _output_get (Variables|Default|SetHealth 1e+03))
  (Variables|Default|SetMaxHealth _output_get)
  (CallFunction|SetHealthbar))

(event Custom|Turret%20Attack
  (bind _barrel_1 (Variables|Default|GetBarrel%201))
  (bind _barrel_2 (Variables|Default|GetBarrel%202))
  (bind _returnvalue (Transformation|GetWorldTransform _barrel_2))
  (bind _returnvalue_2 (Transformation|GetWorldTransform _barrel_1))
  (Utilities|FlowControl|Delay 2.0)
  (Game|SpawnActorfromClass "/Game/Blueprints/Projectiles/Enemy/BP_enemy_ranged_projectile.BP_enemy_ranged_projectile_C" (Math|Transform|MakeTransform (.location _returnvalue_2) (.rotation _returnvalue_2) "3.000000,3.000000,3.000000") "Undefined" 0 0)
  (Audio|PlaySoundatLocation "/Game/Audio/Effects/Guns/Shooting/C_rocket_launcher_fire.C_rocket_launcher_fire" (.location _returnvalue_2) "0, 0, 0" 1.0 1.0 0.0 0 0 0)
  (Utilities|FlowControl|Delay 0.5)
  (Game|SpawnActorfromClass "/Game/Blueprints/Projectiles/Enemy/BP_enemy_ranged_projectile.BP_enemy_ranged_projectile_C" (Math|Transform|MakeTransform (.location _returnvalue) (.rotation _returnvalue) "3.000000,3.000000,3.000000") "Undefined" 0 0)
  (Audio|PlaySoundatLocation "/Game/Audio/Effects/Guns/Shooting/C_rocket_launcher_fire.C_rocket_launcher_fire" (.location _returnvalue) "0, 0, 0" 1.0 1.0 0.0 0 0 0))

(event Custom|Show%20Health%20Bar
  (if (== (Variables|Default|GetHealthBar) 0)
    (bind _returnvalue (UserInterface|CreateWidget "/Game/Blueprints/UMG/UI_bossHealth.UI_bossHealth_C"))
    (bind _output_get (Variables|Default|SetHealthBar _returnvalue))
    (CallFunction|SetHealthbar)
    (UserInterface|Viewport|AddtoViewport _output_get 0)))

(event EventTick
  (params (DeltaSeconds :type Float%20%28single-precision%29))
  (Variables|Default|SetDeltaSeconds DeltaSeconds)
  (if (Variables|Default|GetIsDead)
    (CallFunction|Death)
    (else
      (bind _asfirst_person_character (Utilities|Casting|CastToFirstPersonCharacter (Game|GetPlayerCharacter 0)))
      (if (Variables|/Game/Blueprints/Characters/FirstPersonCharacter.FirstPersonCharacter_C|GetIsDead _asfirst_person_character)
        (Utilities|FlowControl|DoOnce false :!label _label
          (:Completed
            (CallFunction|Reset)
            (goto _label Reset)))))))

(event Game|Damage|EventAnyDamage
  (params (Damage :type Float%20%28single-precision%29) (DamageType :type Damage%20Type%20Object%20Reference) (InstigatedBy :type Controller%20Object%20Reference) (DamageCauser :type Actor%20Object%20Reference))
  (Variables|Default|SetHealth (- (Variables|Default|GetHealth) Damage))
  (CallFunction|SetHealthbar)
  (CallFunction|HitSound)
  (if (<= (Variables|Default|GetHealth) 0.0)
    (Variables|Default|SetIsDead true)))

(fn ConstructionScript)

(fn SetHealthbar
  (bind _asui_boss_health (Utilities|Casting|CastToUI_bossHealth (Variables|Default|GetHealthBar)))
  (Variables|/Game/Blueprints/UMG/UI_bossHealth.UI_bossHealth_C|SetBossHealth _asui_boss_health (Variables|Default|GetHealth))
  (Variables|/Game/Blueprints/UMG/UI_bossHealth.UI_bossHealth_C|SetBossMaxHealth _asui_boss_health (Variables|Default|GetMaxHealth)))