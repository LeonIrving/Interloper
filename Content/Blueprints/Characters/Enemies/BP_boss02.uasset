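; Multi-phase boss that turns toward the player, fires sniper projectiles after a delay on sight, and shows a health bar.
; Each depleted health pool hides a shell, refills higher, removes an arena floor and spawns ranged enemies, then grenadiers, at random navigable points.
; Player death resets boss and arena and destroys spawned minions.
; Final defeat moves the boss to DeathPoint and spawns a Hub portal and waypoint.
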(event OnSeePawn(PawnSensing)
  (params (Pawn :type Pawn%20Object%20Reference))
  (if (not (Variables|Default|GetIsDead))
    (CallFunction|PrimaryAttack)
    (CallFunction|ShowHealthBar)))

(event Custom|Show%20Health%20Bar
  (if (== (Variables|Default|GetHealthBar) 0)
    (bind _returnvalue (UserInterface|CreateWidget "/Game/Blueprints/UMG/UI_bossHealth.UI_bossHealth_C"))
    (bind _output_get (Variables|Default|SetHealthBar _returnvalue))
    (CallFunction|SetHealthbar)
    (UserInterface|Viewport|AddtoViewport _output_get 0)))

(event Custom|Primary%20Attack
  (Utilities|FlowControl|Delay 1.0)
  (Game|SpawnActorfromClass "/Game/Blueprints/Projectiles/Enemy/BP_enemy_sniper_projectile.BP_enemy_sniper_projectile_C" (Transformation|GetWorldTransform (Variables|Default|GetBulletSpawn)) "Undefined" 0 0)
  (Audio|PlaySoundatLocation "/Game/Audio/Effects/Guns/C_rifle_shoot_large.C_rifle_shoot_large" (Transformation|GetActorLocation) "0, 0, 0" 0.5 1.0 0.0 0 0 0))

(event Custom|Death
  (bind _returnvalue (Transformation|GetActorTransform))
  (Utilities|FlowControl|DoOnce false
    (:Completed
      (Transformation|SetActorTransform (Transformation|GetWorldTransform (Variables|Default|GetDeathPoint)))
      (Rendering|SetVisibility (Variables|Default|GetShell01) true true)
      (bind _returnvalue_2 (Game|SpawnActorfromClass "/Game/Blueprints/Environment/Doors/BP_level_portal_box.BP_level_portal_box_C" (Math|Transform|MakeTransform (.location _returnvalue) (.rotation _returnvalue) "5.000000,5.000000,1") "Undefined" 0 0))
      (bind _output_get (Variables|Default|SetPortal _returnvalue_2))
      (Variables|/Game/Blueprints/Environment/Doors/BP_level_portal_box.BP_level_portal_box_C|SetLevelToLoad _output_get "Hub")
      (Game|SpawnActorfromClass "/Game/Blueprints/Objectives/BP_single_waypoint.BP_single_waypoint_C" (Math|Transform|MakeTransform (Transformation|GetActorLocation) "0, 0, 0" "1,1,1") "Undefined" 0 0))))

(event Custom|Reset
  (bind _arena (Variables|Default|GetArena))
  (bind _output_get (Variables|Default|SetHealth 1e+03))
  (Variables|Default|SetMaxHealth _output_get)
  (Variables|Default|SetPhase 0)
  (Rendering|SetVisibility (Variables|/Game/Blueprints/Environment/Arenas/BP_boss02_arena.BP_boss02_arena_C|GetDefaultSceneRoot _arena) true true)
  (Collision|SetCollisionEnabled (Variables|/Game/Blueprints/Environment/Arenas/BP_boss02_arena.BP_boss02_arena_C|GetFloor%201 _arena) "QueryAndPhysics")
  (Collision|SetCollisionEnabled (Variables|/Game/Blueprints/Environment/Arenas/BP_boss02_arena.BP_boss02_arena_C|GetFloor%202 _arena) "QueryAndPhysics")
  (Collision|SetCollisionEnabled (Variables|/Game/Blueprints/Environment/Arenas/BP_boss02_arena.BP_boss02_arena_C|GetFloor%203 _arena) "QueryAndPhysics")
  (Rendering|SetVisibility (Variables|Default|GetDefaultSceneRoot) true true)
  (CallFunction|SetHealthbar)
  (for _array_element (Variables|Default|GetEnemies)
    (Actor|DestroyActor _array_element)))

(event Custom|Spawn%20Enemy
  (params (Enemy :type BP%20Base%20Enemy%20Class%20Reference) (Radius :type Float%20%28single-precision%29))
  (bind _returnvalue (Transformation|GetActorLocation))
  (bind _randomlocation (Class|NavigationSystemV1|GetRandomPointinNavigableRadius (Math|Vector|MakeVector (.x _returnvalue) (.y _returnvalue) (.z _returnvalue)) Radius 0 0))
  (bind _returnvalue_2 (AI|SpawnAIFromClass Enemy 0 (Math|Vector|MakeVector (.x _randomlocation) (.y _randomlocation) (+ (.z _returnvalue) -6e+02)) "0, 0, 0" false))
  (Utilities|Array|Add (Variables|Default|GetEnemies) _returnvalue_2))

(event EventTick
  (params (DeltaSeconds :type Float%20%28single-precision%29))
  (if (Variables|Default|GetIsDead)
    (CallFunction|Death)
    (else
      (bind _asfirst_person_character (Utilities|Casting|CastToFirstPersonCharacter (Game|GetPlayerCharacter 0)))
      (Transformation|SetWorldRotation (Variables|Default|GetDefaultSceneRoot) (Math|Rotator|MakeRotator 0.0 0.0 (.yaw (Math|Rotator|FindLookatRotation (Transformation|GetActorLocation) (Transformation|GetActorLocation _asfirst_person_character)))) false false)
      (Transformation|SetWorldRotation (Variables|Default|GetBulletSpawn) (Math|Rotator|MakeRotator (.roll (Math|Rotator|FindLookatRotation (Transformation|GetActorLocation) (Transformation|GetActorLocation _asfirst_person_character))) (.pitch (Math|Rotator|FindLookatRotation (Transformation|GetActorLocation) (Transformation|GetActorLocation _asfirst_person_character))) (.yaw (Math|Rotator|FindLookatRotation (Transformation|GetActorLocation) (Transformation|GetActorLocation _asfirst_person_character)))) false false)
      (if (Variables|/Game/Blueprints/Characters/FirstPersonCharacter.FirstPersonCharacter_C|GetIsDead _asfirst_person_character)
        (Utilities|FlowControl|DoOnce false :!label _label
          (:Completed
            (CallFunction|Reset)
            (goto _label Reset)))))))

(event Game|Damage|EventAnyDamage
  (params (Damage :type Float%20%28single-precision%29) (DamageType :type Damage%20Type%20Object%20Reference) (InstigatedBy :type Controller%20Object%20Reference) (DamageCauser :type Actor%20Object%20Reference))
  (bind _arena (Variables|Default|GetArena))
  (bind _arena_2 (Variables|Default|GetArena))
  (bind _floor_3 (Variables|/Game/Blueprints/Environment/Arenas/BP_boss02_arena.BP_boss02_arena_C|GetFloor%203 _arena))
  (bind _floor_2 (Variables|/Game/Blueprints/Environment/Arenas/BP_boss02_arena.BP_boss02_arena_C|GetFloor%202 _arena_2))
  (Variables|Default|SetHealth (- (Variables|Default|GetHealth) Damage))
  (CallFunction|SetHealthbar)
  (if (<= (Variables|Default|GetHealth) 0.0)
    ;[0 0 0] Phase 2
    (if (== (Variables|Default|GetPhase) 0)
      (Variables|Default|SetPhase 1)
      (Rendering|SetVisibility (Variables|Default|GetShell01) false false)
      (bind _output_get (Variables|Default|SetHealth 1.5e+03))
      (Variables|Default|SetMaxHealth _output_get)
      (Collision|SetCollisionEnabled _floor_3 "NoCollision")
      (Rendering|SetVisibility _floor_3 false false)
      (CallFunction|SetHealthbar)
      (CallFunction|SpawnEnemy "/Game/Blueprints/Characters/Enemies/BP_enemy_ranged.BP_enemy_ranged_C" 4e+03)
      (CallFunction|SpawnEnemy "/Game/Blueprints/Characters/Enemies/BP_enemy_ranged.BP_enemy_ranged_C" 4e+03)
      (CallFunction|SpawnEnemy "/Game/Blueprints/Characters/Enemies/BP_enemy_ranged.BP_enemy_ranged_C" 4e+03)
      (else
        ;[0 0 0] Phase 3
        (if (== (Variables|Default|GetPhase) 1)
          (Variables|Default|SetPhase 2)
          (Rendering|SetVisibility (Variables|Default|GetShell02) false false)
          (bind _output_get_2 (Variables|Default|SetHealth 2e+03))
          (Variables|Default|SetMaxHealth _output_get_2)
          (Collision|SetCollisionEnabled _floor_2 "NoCollision")
          (Rendering|SetVisibility _floor_2 false false)
          (CallFunction|SetHealthbar)
          (CallFunction|SpawnEnemy "/Game/Blueprints/Characters/Enemies/BP_enemy_grenadier.BP_enemy_grenadier_C" 2e+03)
          (CallFunction|SpawnEnemy "/Game/Blueprints/Characters/Enemies/BP_enemy_grenadier.BP_enemy_grenadier_C" 2e+03)
          (CallFunction|SpawnEnemy "/Game/Blueprints/Characters/Enemies/BP_enemy_grenadier.BP_enemy_grenadier_C" 2e+03)
          (else
            (Variables|Default|SetIsDead true)))))))

(fn ConstructionScript)

(fn SetHealthbar
  (bind _asui_boss_health (Utilities|Casting|CastToUI_bossHealth (Variables|Default|GetHealthBar)))
  (Variables|/Game/Blueprints/UMG/UI_bossHealth.UI_bossHealth_C|SetBossHealth _asui_boss_health (Variables|Default|GetHealth))
  (Variables|/Game/Blueprints/UMG/UI_bossHealth.UI_bossHealth_C|SetBossMaxHealth _asui_boss_health (Variables|Default|GetMaxHealth)))