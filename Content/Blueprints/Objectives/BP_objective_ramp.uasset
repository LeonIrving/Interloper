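; Objective ramp actor that lowers itself once four referenced capture plates are all captured.
; BeginPlay stores its world location as the start and a point 1000 units below as the end.
; When Triggered finds every plate captured, a Movement timeline lerps between them, applying the result as relative location.
; When the timeline finishes, it spawns a BP_single_waypoint at the original position.
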(event Custom|Triggered
  (bind _start (Variables|Default|GetStart))
  (if (Math|Boolean|ANDBoolean (Variables|/Game/Blueprints/Objectives/BP_capture_plate.BP_capture_plate_C|GetCaptured (Variables|Default|GetCapturePlate1)) (Variables|/Game/Blueprints/Objectives/BP_capture_plate.BP_capture_plate_C|GetCaptured (Variables|Default|GetCapturePlate2)) (Variables|/Game/Blueprints/Objectives/BP_capture_plate.BP_capture_plate_C|GetCaptured (Variables|Default|GetCapturePlate3)) (Variables|/Game/Blueprints/Objectives/BP_capture_plate.BP_capture_plate_C|GetCaptured (Variables|Default|GetCapturePlate4)))
    (bind _alpha (Timeline|Movement Play)
      (:Update
        (Transformation|SetActorRelativeLocation (Math|Vector|Lerp(Vector) _start (Variables|Default|GetEnd) _alpha)))
      (:Finished
        (Game|SpawnActorfromClass "/Game/Blueprints/Objectives/BP_single_waypoint.BP_single_waypoint_C" (Math|Transform|MakeTransform _start "0, 0, 0" "1,1,1") "Undefined" 0 0)))))

(event EventBeginPlay
  (bind _returnvalue (Transformation|GetActorLocation))
  (Variables|Default|SetStart (Math|Vector|MakeVector (.x _returnvalue) (.y _returnvalue) (.z _returnvalue)))
  (Variables|Default|SetEnd (Math|Vector|MakeVector (.x _returnvalue) (.y _returnvalue) (+ (.z _returnvalue) -1e+03))))

(fn ConstructionScript)