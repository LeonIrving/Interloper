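; Key lock objective that opens a linked door and destroys itself when the player interacts with all required keys collected.
; An objective trigger posts the key count once and reveals three key waypoints.
; AddKey increments the count, updates the objective text and reveals the lock's waypoint once the requirement is met.
; The interact radius toggles input and the HUD prompt; interacting without the required keys reposts the objective.
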(event OnComponentBeginOverlap(InteractRadius)
  (params (OverlappedComponent :type Primitive%20Component%20Object%20Reference) (OtherActor :type Actor%20Object%20Reference) (OtherComp :type Primitive%20Component%20Object%20Reference) (OtherBodyIndex :type Integer) (bFromSweep :type Boolean) (SweepResult :type Hit%20Result%20Structure%20%28by%20ref%29))
  (bind _asfirst_person_character (Utilities|Casting|CastToFirstPersonCharacter OtherActor))
  (Input|EnableInput (Game|GetPlayerController 0))
  (Default|ShowPrompt (Variables|/Game/Blueprints/Characters/FirstPersonCharacter.FirstPersonCharacter_C|GetHUD _asfirst_person_character)))

(event OnComponentEndOverlap(InteractRadius)
  (params (OverlappedComponent :type Primitive%20Component%20Object%20Reference) (OtherActor :type Actor%20Object%20Reference) (OtherComp :type Primitive%20Component%20Object%20Reference) (OtherBodyIndex :type Integer))
  (Utilities|Casting|CastToFirstPersonCharacter OtherActor)
  (Input|DisableInput (Game|GetPlayerController 0))
  (Default|HidePrompt (Variables|/Game/Blueprints/Characters/FirstPersonCharacter.FirstPersonCharacter_C|GetHUD (stale OnComponentBeginOverlap(InteractRadius) _asfirst_person_character))))

(event OnComponentBeginOverlap(ObjectiveCollision)
  (params (OverlappedComponent :type Primitive%20Component%20Object%20Reference) (OtherActor :type Actor%20Object%20Reference) (OtherComp :type Primitive%20Component%20Object%20Reference) (OtherBodyIndex :type Integer) (bFromSweep :type Boolean) (SweepResult :type Hit%20Result%20Structure%20%28by%20ref%29))
  (Utilities|Casting|CastToFirstPersonCharacter OtherActor)
  (Utilities|FlowControl|DoOnce false
    (:Completed
      (CallFunction|ShowObjective)
      (Rendering|SetVisibility (Variables|/Game/Blueprints/Objectives/BP_objective_key.BP_objective_key_C|GetWaypoint (Variables|Default|GetKey%201)) true false)
      (Rendering|SetVisibility (Variables|/Game/Blueprints/Objectives/BP_objective_key.BP_objective_key_C|GetWaypoint (Variables|Default|GetKey%202)) true false)
      (Rendering|SetVisibility (Variables|/Game/Blueprints/Objectives/BP_objective_key.BP_objective_key_C|GetWaypoint (Variables|Default|GetKey%203)) true false))))

(event Custom|Show%20Objective
  (bind _asfirst_person_character (Utilities|Casting|CastToFirstPersonCharacter (Game|GetPlayerCharacter 0)))
  (Variables|Default|SetObjectiveText (Utilities|Text|FormatText "Keys Collected: {Player Keys} / {Required Keys}" (Variables|Default|GetPlayerKeys) (Variables|Default|GetRequiredKeys)))
  (Default|AddObjective (Variables|/Game/Blueprints/Characters/FirstPersonCharacter.FirstPersonCharacter_C|GetObjectives _asfirst_person_character) (Variables|Default|GetObjectiveText)))

(event Input|ActionEvents|InputActionInteract
  (params (Key :type Key%20Structure))
  (:Pressed
    (if (== (Variables|Default|GetPlayerKeys) (Variables|Default|GetRequiredKeys))
      (Default|Open (Variables|Default|GetDoor))
      (Actor|DestroyActor)
      (else
        (CallFunction|ShowObjective)))))

(fn ConstructionScript)

(fn AddKey
  (bind _result (Math|Integer|IncrementInt (Variables|Default|GetPlayerKeys))
    (:%20%20
      (Variables|Default|SetObjectiveText (Utilities|Text|FormatText "Keys Collected: {Player Keys} / {Required Keys}" _result (Variables|Default|GetRequiredKeys)))
      (bind _asfirst_person_character (Utilities|Casting|CastToFirstPersonCharacter (Game|GetPlayerCharacter 0)))
      (if (!= (Variables|Default|GetPlayerKeys) (Variables|Default|GetRequiredKeys))
        (Default|AddObjective (Variables|/Game/Blueprints/Characters/FirstPersonCharacter.FirstPersonCharacter_C|GetObjectives _asfirst_person_character) (Variables|Default|GetObjectiveText))
        (else
          (Default|AddObjective (Variables|/Game/Blueprints/Characters/FirstPersonCharacter.FirstPersonCharacter_C|GetObjectives _asfirst_person_character) (Variables|Default|GetObjectiveText))
          (Rendering|SetVisibility (Variables|Default|GetWaypoint) true false))))))