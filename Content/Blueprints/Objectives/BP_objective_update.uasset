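; Objective trigger actor that hands the player a new objective and shows a waypoint marker for it.
; The first overlap of the FirstPersonCharacter with Collision adds ObjectiveText to the character's Objectives and makes the Waypoint visible, guarded by a DoOnce.
; A separate WaypointCollision hides the Waypoint whenever the character overlaps it.
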(event OnComponentBeginOverlap(WaypointCollision)
  (params (OverlappedComponent :type Primitive%20Component%20Object%20Reference) (OtherActor :type Actor%20Object%20Reference) (OtherComp :type Primitive%20Component%20Object%20Reference) (OtherBodyIndex :type Integer) (bFromSweep :type Boolean) (SweepResult :type Hit%20Result%20Structure%20%28by%20ref%29))
  (Utilities|Casting|CastToFirstPersonCharacter OtherActor)
  (Rendering|SetVisibility (Variables|Default|GetWaypoint) false false))

(event OnComponentBeginOverlap(Collision)
  (params (OverlappedComponent :type Primitive%20Component%20Object%20Reference) (OtherActor :type Actor%20Object%20Reference) (OtherComp :type Primitive%20Component%20Object%20Reference) (OtherBodyIndex :type Integer) (bFromSweep :type Boolean) (SweepResult :type Hit%20Result%20Structure%20%28by%20ref%29))
  (bind _asfirst_person_character (Utilities|Casting|CastToFirstPersonCharacter OtherActor))
  (Utilities|FlowControl|DoOnce false
    (:Completed
      (Default|AddObjective (Variables|/Game/Blueprints/Characters/FirstPersonCharacter.FirstPersonCharacter_C|GetObjectives _asfirst_person_character) (Variables|Default|GetObjective%20Text))
      (Rendering|SetVisibility (Variables|Default|GetWaypoint) true false))))

(fn ConstructionScript)