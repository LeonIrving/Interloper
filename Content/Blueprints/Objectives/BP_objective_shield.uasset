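; BP_objective_shield is an objective shield that shuts down once both of its linked cores are triggered.
; Its Deactivate event checks the IsTriggered state of Core1 and Core2 and does nothing unless both are set.
; When both are, it plays an engine shutdown sound, spawns a BP_single_waypoint at its own location and destroys itself.
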(event Custom|Deactivate
  (if (and (Variables|/Game/Blueprints/Objectives/BP_shootable_core.BP_shootable_core_C|GetisTriggered (Variables|Default|GetCore1)) (Variables|/Game/Blueprints/Objectives/BP_shootable_core.BP_shootable_core_C|GetisTriggered (Variables|Default|GetCore2)))
    (Audio|PlaySoundatLocation "/Game/Audio/Effects/Objectives/sfx_engine_shutdown_1.sfx_engine_shutdown_1" (Transformation|GetActorLocation) "0, 0, 0" 0.5 1.0 0.0 0 0 0)
    (Game|SpawnActorfromClass "/Game/Blueprints/Objectives/BP_single_waypoint.BP_single_waypoint_C" (Math|Transform|MakeTransform (Transformation|GetActorLocation) "0, 0, 0" "1,1,1") "Undefined" 0 0)
    (Actor|DestroyActor)))

(fn ConstructionScript)