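; Collectible objective key that the player picks up to add a key to its linked BP_objective_key_lock.
; Overlapping the InteractRadius with the FirstPersonCharacter enables input on the key and shows a HUD prompt; leaving reverses both.
; Pressing Interact calls AddKey on the actor in the Lock reference and then destroys the key.
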(event OnComponentBeginOverlap(InteractRadius)
  (params (OverlappedComponent :type Primitive%20Component%20Object%20Reference) (OtherActor :type Actor%20Object%20Reference) (OtherComp :type Primitive%20Component%20Object%20Reference) (OtherBodyIndex :type Integer) (bFromSweep :type Boolean) (SweepResult :type Hit%20Result%20Structure%20%28by%20ref%29))
  (bind _asfirst_person_character (Utilities|Casting|CastToFirstPersonCharacter OtherActor))
  (Input|EnableInput (Game|GetPlayerController 0))
  (Default|ShowPrompt (Variables|/Game/Blueprints/Characters/FirstPersonCharacter.FirstPersonCharacter_C|GetHUD _asfirst_person_character)))

(event OnComponentEndOverlap(InteractRadius)
  (params (OverlappedComponent :type Primitive%20Component%20Object%20Reference) (OtherActor :type Actor%20Object%20Reference) (OtherComp :type Primitive%20Component%20Object%20Reference) (OtherBodyIndex :type Integer))
  (Utilities|Casting|CastToFirstPersonCharacter OtherActor)
  (Input|DisableInput (Game|GetPlayerController 0))
  (Default|HidePrompt (Variables|/Game/Blueprints/Characters/FirstPersonCharacter.FirstPersonCharacter_C|GetHUD (stale OnComponentBeginOverlap(InteractRadius) _asfirst_person_character))))

(event Input|ActionEvents|InputActionInteract
  (params (Key :type Key%20Structure))
  (:Pressed
    (bind _asbp_objective_key_lock (Utilities|Casting|CastToBP_objective_key_lock (Variables|Default|GetLock)))
    (Default|AddKey _asbp_objective_key_lock)
    (Actor|DestroyActor)))

(fn ConstructionScript)