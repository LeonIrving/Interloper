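; Capture plate objective that the first-person character captures by staying inside its sphere trigger, which then triggers a linked ramp.
; Sphere overlaps set CanCapture; each tick until captured, this plays or reverses the CaptureProgress timeline, so progress drains when the player leaves.
; The spotlight shows red when idle, orange while capturing and green once captured.
; Completion locks the plate, plays a capture sound and calls Triggered on the ramp.
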(event OnComponentBeginOverlap(Sphere)
  (params (OverlappedComponent :type Primitive%20Component%20Object%20Reference) (OtherActor :type Actor%20Object%20Reference) (OtherComp :type Primitive%20Component%20Object%20Reference) (OtherBodyIndex :type Integer) (bFromSweep :type Boolean) (SweepResult :type Hit%20Result%20Structure%20%28by%20ref%29))
  (Utilities|Casting|CastToFirstPersonCharacter OtherActor)
  (Variables|Default|SetCanCapture true))

(event OnComponentEndOverlap(Sphere)
  (params (OverlappedComponent :type Primitive%20Component%20Object%20Reference) (OtherActor :type Actor%20Object%20Reference) (OtherComp :type Primitive%20Component%20Object%20Reference) (OtherBodyIndex :type Integer))
  (Utilities|Casting|CastToFirstPersonCharacter OtherActor)
  (Variables|Default|SetCanCapture false))

(event EventTick
  (params (DeltaSeconds :type Float%20%28single-precision%29))
  (bind _spotlight (Variables|Default|GetSpotLight))
  (if (not (Variables|Default|GetCaptured))
    (if (Variables|Default|GetCanCapture)
      (Rendering|Components|Light|SetLightColor _spotlight "(R=1.000000,G=0.633649,B=0.000000,A=1.000000)" true)
      (bind _progress (Timeline|Capture%20Progress Play)
        (:Update
          (bind _output_get (Variables|Default|SetCaptureProgress _progress))
          (if (== _output_get 1.0)
            (Variables|Default|SetCaptured true)
            (Rendering|Components|Light|SetLightColor (Variables|Default|GetSpotLight) "(R=0.007036,G=1.000000,B=0.000000,A=1.000000)" true)
            (Audio|PlaySoundatLocation "/Game/Audio/Effects/Objectives/Point_Capture.Point_Capture" (Transformation|GetActorLocation) "0, 0, 0" 1.5 1.0 0.0 0 0 0)
            (Default|Triggered (Variables|Default|GetRamp)))))
      (else
        (Rendering|Components|Light|SetLightColor _spotlight "(R=1.000000,G=0.000000,B=0.014766,A=1.000000)" true)
        (Timeline|Capture%20Progress Reverse)))))

(fn ConstructionScript)