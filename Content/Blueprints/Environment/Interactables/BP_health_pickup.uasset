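; BP_health_pickup is a health pickup that heals a FirstPersonCharacter overlapping its collision component.
; It sets Health to MaxHealth when Health plus Amount is at least zero, so it normally fully heals, and only adds Amount otherwise.
; It then spawns the M_bulletExplosion01 emitter and A_Heal sound at its location and destroys itself.
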(event OnComponentBeginOverlap(Collision)
  (params (OverlappedComponent :type Primitive%20Component%20Object%20Reference) (OtherActor :type Actor%20Object%20Reference) (OtherComp :type Primitive%20Component%20Object%20Reference) (OtherBodyIndex :type Integer) (bFromSweep :type Boolean) (SweepResult :type Hit%20Result%20Structure%20%28by%20ref%29))
  (bind _returnvalue (Transformation|GetActorTransform))
  (bind _asfirst_person_character (Utilities|Casting|CastToFirstPersonCharacter OtherActor))
  (if (>= (+ (Variables|/Game/Blueprints/Characters/FirstPersonCharacter.FirstPersonCharacter_C|GetHealth _asfirst_person_character) (Variables|Default|GetAmount)) 0.0)
    (Variables|/Game/Blueprints/Characters/FirstPersonCharacter.FirstPersonCharacter_C|SetHealth _asfirst_person_character (Variables|/Game/Blueprints/Characters/FirstPersonCharacter.FirstPersonCharacter_C|GetMaxHealth _asfirst_person_character))
    (else
      (Variables|/Game/Blueprints/Characters/FirstPersonCharacter.FirstPersonCharacter_C|SetHealth _asfirst_person_character (+ (Variables|/Game/Blueprints/Characters/FirstPersonCharacter.FirstPersonCharacter_C|GetHealth _asfirst_person_character) (Variables|Default|GetAmount)))))
  (Effects|SpawnEmitteratLocation "/Game/Particles/M_bulletExplosion01.M_bulletExplosion01" (.location _returnvalue) (.rotation _returnvalue))
  (Audio|PlaySoundatLocation "/Game/Audio/Effects/A_Heal.A_Heal" (.location _returnvalue) "0, 0, 0" 1.0 1.0 0.0 0 0 0)
  (Actor|DestroyActor))

(fn ConstructionScript)