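; BP_elevator is an interactable elevator that makes a one-way trip when the player uses it.
; The Collision overlap enables input and shows a HUD prompt for a FirstPersonCharacter while IsActive is true; leaving reverses both.
; Interact clears IsActive, hides the prompt and plays the Movement timeline.
; The timeline lerps the actor's relative location, without sweep, between world positions cached at BeginPlay from the actor and its End component.
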(event OnComponentBeginOverlap(Collision)
  (params (OverlappedComponent :type Primitive%20Component%20Object%20Reference) (OtherActor :type Actor%20Object%20Reference) (OtherComp :type Primitive%20Component%20Object%20Reference) (OtherBodyIndex :type Integer) (bFromSweep :type Boolean) (SweepResult :type Hit%20Result%20Structure%20%28by%20ref%29))
  (if (Variables|Default|GetIsActive)
    (bind _asfirst_person_character (Utilities|Casting|CastToFirstPersonCharacter OtherActor))
    (Input|EnableInput (Game|GetPlayerController 0))
    (Default|ShowPrompt (Variables|/Game/Blueprints/Characters/FirstPersonCharacter.FirstPersonCharacter_C|GetHUD _asfirst_person_character))))

(event OnComponentEndOverlap(Collision)
  (params (OverlappedComponent :type Primitive%20Component%20Object%20Reference) (OtherActor :type Actor%20Object%20Reference) (OtherComp :type Primitive%20Component%20Object%20Reference) (OtherBodyIndex :type Integer))
  (bind _asfirst_person_character (Utilities|Casting|CastToFirstPersonCharacter OtherActor))
  (Input|DisableInput (Game|GetPlayerController 0))
  (Default|HidePrompt (Variables|/Game/Blueprints/Characters/FirstPersonCharacter.FirstPersonCharacter_C|GetHUD _asfirst_person_character)))

(event EventBeginPlay
  (Variables|Default|SetStartLocation (Transformation|GetActorLocation))
  (Variables|Default|SetEndLocation (Transformation|GetWorldLocation (Variables|Default|GetEnd))))

(event Input|ActionEvents|InputActionInteract
  (params (Key :type Key%20Structure))
  (:Pressed
    (Input|DisableInput (Game|GetPlayerController 0))
    (Default|HidePrompt (Variables|/Game/Blueprints/Characters/FirstPersonCharacter.FirstPersonCharacter_C|GetHUD (stale OnComponentBeginOverlap(Collision) _asfirst_person_character)))
    (Variables|Default|SetIsActive false)
    (bind _alpha (Timeline|Movement Play)
      (:Update
        (Transformation|SetActorRelativeLocation (Math|Vector|Lerp(Vector) (Variables|Default|GetStartLocation) (Variables|Default|GetEndLocation) _alpha))))))

(fn ConstructionScript)