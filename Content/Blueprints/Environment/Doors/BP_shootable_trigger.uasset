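; Shootable trigger in the Doors environment set that explodes when damaged enough and flags itself as triggered.
; Each AnyDamage hit lowers Health and plays a 2D hitmarker sound.
; Damage is compared with the already reduced Health, so it fires once a hit is at least the remaining value.
; Firing sets CanTrigger, spawns an explosion effect and sound at the mesh, destroys the mesh, then sets IsTriggered.
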(event Game|Damage|EventAnyDamage
  (params (Damage :type Float%20%28single-precision%29) (DamageType :type Damage%20Type%20Object%20Reference) (InstigatedBy :type Controller%20Object%20Reference) (DamageCauser :type Actor%20Object%20Reference))
  (bind _mesh (Variables|Default|GetMesh))
  (bind _returnvalue (Transformation|GetWorldTransform _mesh))
  (Variables|Default|SetHealth (- (Variables|Default|GetHealth) Damage))
  (Audio|PlaySound2D "/Game/Audio/Effects/Guns/A_Hitmarker.A_Hitmarker" 1.0 1.0 0.0 0 0)
  (if (>= Damage (Variables|Default|GetHealth))
    (Variables|Default|SetcanTrigger true)
    (Effects|SpawnEmitteratLocation "/Game/Particles/P_Explosion2.P_Explosion2" (.location _returnvalue) (.rotation _returnvalue) (.scale _returnvalue))
    (Audio|PlaySoundatLocation "/Game/Audio/Effects/A_Small_Explosion.A_Small_Explosion" (.location _returnvalue) "0, 0, 0" 1.0 1.0 0.0 0 0 0)
    (Components|DestroyComponent _mesh)
    (Variables|Default|SetisTriggered true)))

(fn ConstructionScript)