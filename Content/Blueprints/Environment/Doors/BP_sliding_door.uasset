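; Sliding door that lowers out of the way when the player approaches and switches the level from ambient to boss music.
; Overlapping the trigger box with FirstPersonCharacter plays a timeline that drives the cube's relative Z downward, and leaving reverses it.
; The first entry only, gated by DoOnce, crossfades the referenced AmbientMusic and BossMusic actors and plays the door-opening sound at the door's location.
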(event OnComponentEndOverlap(Box)
  (params (OverlappedComponent :type Primitive%20Component%20Object%20Reference) (OtherActor :type Actor%20Object%20Reference) (OtherComp :type Primitive%20Component%20Object%20Reference) (OtherBodyIndex :type Integer))
  (Utilities|Casting|CastToFirstPersonCharacter OtherActor)
  (bind _alpha (Timeline|Movement Reverse)
    (:Update
      (Transformation|SetRelativeLocation (Variables|Default|GetCube) (Math|Vector|MakeVector 0.0 0.0 (* _alpha -1e+03)) false false))))

(event OnComponentBeginOverlap(Box)
  (params (OverlappedComponent :type Primitive%20Component%20Object%20Reference) (OtherActor :type Actor%20Object%20Reference) (OtherComp :type Primitive%20Component%20Object%20Reference) (OtherBodyIndex :type Integer) (bFromSweep :type Boolean) (SweepResult :type Hit%20Result%20Structure%20%28by%20ref%29))
  (Utilities|Casting|CastToFirstPersonCharacter OtherActor)
  (Utilities|FlowControl|Sequence
    (:then_0
      (bind _alpha (Timeline|Movement Play)
        (:Update
          (Transformation|SetRelativeLocation (Variables|Default|GetCube) (Math|Vector|MakeVector 0.0 0.0 (* _alpha -1e+03)) false false))))
    (:then_1
      (Utilities|FlowControl|DoOnce false
        (:Completed
          (Audio|Components|Audio|FadeOut (Variables|/Script/Engine.AmbientSound|GetAudioComponent (Variables|Default|GetAmbientMusic)) 3.0 0.0 :!class /Script/Engine.AudioComponent)
          (Audio|Components|Audio|FadeIn (Variables|/Script/Engine.AmbientSound|GetAudioComponent (Variables|Default|GetBossMusic)) 3.0 1.0 0.0 :!class /Script/Engine.AudioComponent)
          (Audio|PlaySoundatLocation "/Game/Audio/Effects/large_door_open.large_door_open" (Transformation|GetActorLocation) "0, 0, 0" 1.0 1.0 0.0 0 0 0))))))

(fn ConstructionScript)