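; Level portal that sends the player to another level when they enter its sphere.
; On overlap by the FirstPersonCharacter, it creates a loading screen widget if none is cached and passes it the level name and image.
; It then adds the widget to the viewport and immediately opens the target level by name.
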(event OnComponentBeginOverlap(Sphere)
  (params (OverlappedComponent :type Primitive%20Component%20Object%20Reference) (OtherActor :type Actor%20Object%20Reference) (OtherComp :type Primitive%20Component%20Object%20Reference) (OtherBodyIndex :type Integer) (bFromSweep :type Boolean) (SweepResult :type Hit%20Result%20Structure%20%28by%20ref%29))
  (Utilities|Casting|CastToFirstPersonCharacter OtherActor)
  (Utilities|IsValid (Variables|Default|GetLoadingScreen)
    (:Is%20Valid
      _)
    (:Is%20Not%20Valid
      (bind _returnvalue (UserInterface|CreateWidget "/Game/Blueprints/UMG/UI_loading_screen.UI_loading_screen_C"))
      (Variables|Default|SetLoadingScreen _returnvalue)))
  (Variables|/Game/Blueprints/UMG/UI_loading_screen.UI_loading_screen_C|SetLevel%20Name (Variables|Default|GetLoadingScreen) (Variables|Default|GetLevel%20Name))
  (Variables|/Game/Blueprints/UMG/UI_loading_screen.UI_loading_screen_C|SetLevel%20Image (Variables|Default|GetLoadingScreen) (Variables|Default|GetLevel%20Image))
  (UserInterface|Viewport|AddtoViewport (Variables|Default|GetLoadingScreen) 0)
  (Game|OpenLevel(byName) (Variables|Default|GetLevelToLoad)))

(fn ConstructionScript)