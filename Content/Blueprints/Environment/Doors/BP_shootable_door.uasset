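; Door actor that slides upward once its referenced Trigger reports being triggered, presumably by being shot.
; BeginPlay caches the actor's location as Start and a point 2000 units above it as End.
; Tick polls the trigger and plays the DoorMovement timeline, which lerps the actor's relative location between those world-space points without sweep.
; The graph has no logic to close the door.
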(event EventTick
  (params (DeltaSeconds :type Float%20%28single-precision%29))
  (if (Variables|/Game/Blueprints/Environment/Doors/BP_shootable_trigger.BP_shootable_trigger_C|GetisTriggered (Variables|Default|GetTrigger))
    (bind _alpha (Timeline|Door%20Movement Play)
      (:Update
        (Transformation|SetActorRelativeLocation (Math|Vector|Lerp(Vector) (Variables|Default|GetStart) (Variables|Default|GetEnd) _alpha))))))

(event EventBeginPlay
  (bind _returnvalue (Transformation|GetActorLocation))
  (Variables|Default|SetStart (Math|Vector|MakeVector (.x _returnvalue) (.y _returnvalue) (.z _returnvalue)))
  (Variables|Default|SetEnd (Math|Vector|MakeVector (.x _returnvalue) (.y _returnvalue) (+ (.z _returnvalue) 2e+03))))

(fn ConstructionScript)